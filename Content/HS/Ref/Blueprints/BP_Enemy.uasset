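; Enemy that keeps turning to face the player and fires at them on a repeating delay until killed.
; Its gun mesh snaps to a hand socket at construction, and shots spawn from a scene component.
; Hit clears the body mesh, spawns a destructible copy and throws a physical BP_Gun forward with spin.
; The actor lingers for a split second so its colliders smash the destructible, working around APEX damage not working.
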(event `self.ReceiveBeginPlay`
  (set `self.PlayerRef` (`GameplayStatics.GetPlayerPawn` 0))
  (`KismetSystemLibrary.Delay` (`self.TimeBetweenShots`))
  (`self.Fire`))

(event `self.ReceiveTick`
  (params (DeltaSeconds :type "Float (single-precision)"))
  (if (not (`self.bIsDead`))
    (`self.K2_SetActorRotation` (`KismetMathLibrary.FindLookAtRotation` (`self.K2_GetActorLocation`) (`self.K2_GetActorLocation` (`self.PlayerRef`))))))

(event `Fire`
  (bind _returnvalue (`SceneComponent.K2_GetComponentLocation` (`self.Scene`)))
  (bind (_returnvalue_roll _returnvalue_pitch _returnvalue_yaw) (`KismetMathLibrary.BreakRotator` (`KismetMathLibrary.FindLookAtRotation` _returnvalue (`self.K2_GetActorLocation` (`self.PlayerRef`)))))
  (if (not (`self.bIsDead`))
    (`|SpawnActorFromClass` "/Game/HS/Ref/Blueprints/BP_Projectile.BP_Projectile_C" (`KismetMathLibrary.MakeTransform` _returnvalue (`KismetMathLibrary.MakeRotator` _returnvalue_roll 0.0 _returnvalue_yaw)) "AlwaysSpawn" "OverrideRootScale" null null)
    (`KismetSystemLibrary.Delay` (`self.TimeBetweenShots`))
    (`self.Fire`)))

(fn `DestroyEnemy`
  (`self.K2_DestroyActor`))

(fn `Hit`
  (if (not (`self.bIsDead`))
    (set `self.bIsDead` true)
    (`SkinnedMeshComponent.SetSkinnedAssetAndUpdate` (`self.Mesh`) null true)
    (`|SpawnActorFromClass` "/Game/HS/Ref/Blueprints/BP_DestructibleEnemy.BP_DestructibleEnemy_C" (`SceneComponent.K2_GetComponentToWorld` (`self.Mesh`)) "AlwaysSpawn" "OverrideRootScale" null null)
    (bind _returnvalue (`|SpawnActorFromClass` "/Game/HS/Ref/Blueprints/BP_Gun.BP_Gun_C" (`SceneComponent.K2_GetComponentToWorld` (`self.SkeletalMesh`)) "AlwaysSpawn" "OverrideRootScale" null null))
    (`/Game/HS/Ref/Blueprints/BP_Gun.Thrown` _returnvalue)
    (bind _box (`/Game/HS/Ref/Blueprints/BP_Gun.Box` _returnvalue))
    ;[0 0 0] Add small amount of rotation to gun based on adding force at an offset from the objects pivot point.
    (`PrimitiveComponent.AddImpulseAtLocation` _box (50.0 50.0 50.0) (- (`SceneComponent.K2_GetComponentLocation` _box) (0.0 0.0 2.0)) "None")
    ;[0 0 0] Throw the weapon at the player
    (`PrimitiveComponent.AddImpulse` _box (* (+ (`KismetMathLibrary.GetForwardVector` (`SceneComponent.K2_GetComponentRotation` (`self.CapsuleComponent`))) (0.0 0.0 0.2)) (`self.ThrowVelocity`)) "None" true)
    ;[0 0 0] We need the enemy class and its colliders to remain active for a split second as this is what actually causes the spawned destructibleEnemy mesh to smash. Adding damage to the old APEX destruction doesn't seem to work so this is a hacky work around.
    (`KismetSystemLibrary.K2_SetTimer` null "DestroyEnemy" 0.001)))

(fn `UserConstructionScript`
  (`SceneComponent.K2_AttachToComponent` (`self.SkeletalMesh`) (`self.Mesh`) "GunSocket" "SnapToTarget" "SnapToTarget" "SnapToTarget" true))